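; CameraCapture is a Blueprint with a 2D scene capture that mirrors the player's view while leaving out tagged actors.
; On BeginPlay it gathers every actor tagged "NoCapture" once and assigns them as the capture component's hidden actors.
; Every Tick, PositionCamera copies the world transform of player 0's camera manager onto the capture component, without sweep or teleport.
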(event `PositionCamera`
  (`SceneComponent.K2_SetWorldTransform` (`self.SceneCaptureComponent2D`) (`SceneComponent.K2_GetComponentToWorld` (`PlayerCameraManager.TransformComponent` (`GameplayStatics.GetPlayerCameraManager` 0))) false false))

(event `self.ReceiveBeginPlay`
  (bind _outactors (`GameplayStatics.GetAllActorsWithTag` "NoCapture"))
  (set `SceneCaptureComponent.HiddenActors` _outactors (`self.SceneCaptureComponent2D`)))

(event `self.ReceiveTick`
  (params (DeltaSeconds :type "Float (single-precision)"))
  (`self.PositionCamera`))

(fn `UserConstructionScript`)