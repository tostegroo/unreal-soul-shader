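; BP_Mario_High_Soul is a Soul-material variant of the high-detail Mario model that blinks at random and tracks the player camera.
; BeginPlay creates four dynamic eye material instances and assigns them to the Mario mesh.
; Each tick stores the camera location in HeadTarget and randomly triggers a blink.
; A random-speed timeline drives each eye's Blink Amount parameter, with a flag preventing overlapping blinks.
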(event `Set Head Target`
  (set `self.HeadTarget` (`PlayerCameraManager.GetCameraLocation` (`GameplayStatics.GetPlayerCameraManager` 0))))

(event `Blink`
  (if (and (not (`self.IsBlinking`)) (== (`KismetMathLibrary.RandomIntegerInRange` 0 180) 5))
    (set `self.IsBlinking` true)
    (`TimelineComponent.SetPlayRate` (`self.Blink Animation`) (`KismetMathLibrary.RandomFloatInRange` 0.8 3.0))
    (bind (_direction _alpha) (`Timeline|Blink Animation` :!via `PlayFromStart`)
      (:`Update`
        (`MaterialInstanceDynamic.SetScalarParameterValue` (`self.Material_Eye_CL`) "Blink Amount" _alpha)
        (`MaterialInstanceDynamic.SetScalarParameterValue` (`self.Material_Eye_CR`) "Blink Amount" _alpha)
        (`MaterialInstanceDynamic.SetScalarParameterValue` (`self.Material_Eye_R`) "Blink Amount" _alpha)
        (`MaterialInstanceDynamic.SetScalarParameterValue` (`self.Material_Eye_L`) "Blink Amount" _alpha))
      (:`Finished`
        (set `self.IsBlinking` false)))))

(event `self.ReceiveBeginPlay`
  (`|ExecutionSequence`
    (:`then_0`
      (bind _returnvalue (`KismetMaterialLibrary.CreateDynamicMaterialInstance` "/Game/Assets/Geometry/Mario_High/Materials/MI_Mario_Eye_CL_Soul.MI_Mario_Eye_CL_Soul"))
      (set `self.Material_Eye_CL` _returnvalue)
      (bind _returnvalue_2 (`KismetMaterialLibrary.CreateDynamicMaterialInstance` "/Game/Assets/Geometry/Mario_High/Materials/MI_Mario_Eye_CR_Soul.MI_Mario_Eye_CR_Soul"))
      (set `self.Material_Eye_CR` _returnvalue_2)
      (bind _returnvalue_3 (`KismetMaterialLibrary.CreateDynamicMaterialInstance` "/Game/Assets/Geometry/Mario_High/Materials/MI_Mario_Eye_R_Soul.MI_Mario_Eye_R_Soul"))
      (set `self.Material_Eye_R` _returnvalue_3)
      (bind _returnvalue_4 (`KismetMaterialLibrary.CreateDynamicMaterialInstance` "/Game/Assets/Geometry/Mario_High/Materials/MI_Mario_Eye_L_Soul.MI_Mario_Eye_L_Soul"))
      (set `self.Material_Eye_L` _returnvalue_4))
    (:`then_1`
      (`PrimitiveComponent.SetMaterial` (`self.Mario`) 13 (`self.Material_Eye_CL`))
      (`PrimitiveComponent.SetMaterial` (`self.Mario`) 14 (`self.Material_Eye_CR`))
      (`PrimitiveComponent.SetMaterial` (`self.Mario`) 15 (`self.Material_Eye_R`))
      (`PrimitiveComponent.SetMaterial` (`self.Mario`) 2 (`self.Material_Eye_L`)))))

(event `self.ReceiveTick`
  (params (DeltaSeconds :type "Float (single-precision)"))
  (`self.Set Head Target`)
  (`self.Blink`))

(fn `UserConstructionScript`)