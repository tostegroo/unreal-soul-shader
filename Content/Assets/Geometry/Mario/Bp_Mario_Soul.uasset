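; Mario soul Blueprint that blinks at random and keeps a head target on the player's camera.
; BeginPlay creates a dynamic instance of the soul face material and assigns it to the skeletal mesh's second material slot.
; Each tick refreshes HeadTarget from the camera location and randomly may start a blink timeline at varied speed.
; The timeline drives the face material's Phase parameter, with a flag preventing overlapping blinks.
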(event `Set Head Target`
  (set `self.HeadTarget` (`PlayerCameraManager.GetCameraLocation` (`GameplayStatics.GetPlayerCameraManager` 0))))

(event `Blink`
  (if (and (not (`self.IsBlinking`)) (== (`KismetMathLibrary.RandomIntegerInRange` 0 180) 5))
    (set `self.IsBlinking` true)
    (`TimelineComponent.SetPlayRate` (`self.Blink_Animation`) (`KismetMathLibrary.RandomFloatInRange` 1.0 3.0))
    (bind (_direction _alpha) (`Timeline|Blink_Animation` :!via `PlayFromStart`)
      (:`Update`
        (`MaterialInstanceDynamic.SetScalarParameterValue` (`self.Material_Face`) "Phase" _alpha))
      (:`Finished`
        (set `self.IsBlinking` false)))))

(event `self.ReceiveBeginPlay`
  (`|ExecutionSequence`
    (:`then_0`
      (bind _returnvalue (`KismetMaterialLibrary.CreateDynamicMaterialInstance` "/Game/Assets/Geometry/Mario/Materials/MI_Mario_Face_Soul.MI_Mario_Face_Soul"))
      (set `self.Material_Face` _returnvalue))
    (:`then_1`
      (`PrimitiveComponent.SetMaterial` (`self.SkeletalMesh`) 1 (`self.Material_Face`)))))

(event `self.ReceiveTick`
  (params (DeltaSeconds :type "Float (single-precision)"))
  (`self.Blink`)
  (`self.Set Head Target`))

(fn `UserConstructionScript`)